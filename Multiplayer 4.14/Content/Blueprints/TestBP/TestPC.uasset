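; Test player controller that handles character selection, match UI and a per-player kill/death record.
; The selection widget's character ID is resolved to a class through TestGM, then UpdateServer has the game mode swap the character.
; Events manage cursor and input mode, the start message, a FlipFlop-toggled player list, and kill/death increments on the PlayerKD struct.
; The scoreboard logic is disconnected and never runs.
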(event Custom|SetupWidget
  ;[1 1 1] Setup Widget for Choosing character
  (Viewport|RemoveAllWidgets)
  (Variables|Default|SetbShowMouseCursor true)
  (bind _returnvalue (UserInterface|CreateWidget "/Game/UI/TestLevel/ChooseCharacter.ChooseCharacter_C"))
  (bind _output_get (Variables|Default|SetChooseCharacter_WB _returnvalue))
  (UserInterface|Viewport|AddtoViewport _output_get 0)
  (Input|SetInputModeGameandUI self 0 "DoNotLock" true))

(event Custom|GetCharacterID
  (params (CharacterID :type Integer))
  ;[1 1 1] Called from widget / set Character ID var
  (Variables|Default|SetCharacterID CharacterID)
  (CallFunction|GetCharacterClassbyID))

(event Custom|AddPlayerListWidget
  ;[1 1 1] Show / Hide player K/D
  (Utilities|FlowControl|FlipFlop
    (:A
      (bind _returnvalue (UserInterface|CreateWidget "/Game/UI/TestLevel/PlayerList.PlayerList_C"))
      (UserInterface|Viewport|AddtoViewport _returnvalue 0))
    (:B
      (CallFunction|RemovePlayerList))))

(event Custom|RemoveStartMessage
  ;[1 1 1] Set start message and input mode to game
  (Widget|RemovefromParent (stale Custom|InputModeGameOnlyAndAddStartMessage _returnvalue)))

(event Custom|AddDeathToScore
  (bind _playerkd (Variables|Default|GetPlayerKD))
  ;[1 1 1] Add score
  (Utilities|Struct|SetmembersinPlayerKD _playerkd (+ (.Deaths (Utilities|Struct|BreakPlayerKD _playerkd)) 1)))

(event Custom|RemoveScoreboardWB
  ;[1 1 1] Fail to scoreboard
)

(event Custom|FillPlayerClass
  (params (CharacterClass :type Character%20Class%20Reference))
  (bind _playerkd (Variables|Default|GetPlayerKD))
  ;[1 1 1] Fill player Class info
  (Utilities|Struct|SetmembersinPlayerKD _playerkd)
  (CallFunction|UpdateServer _playerkd false))

(event Custom|InputModeGameOnlyAndAddStartMessage
  ;[1 1 1] Set start message and input mode to game
  (Variables|Default|SetbShowMouseCursor false)
  (Input|SetInputModeGameOnly (Game|GetPlayerController 0))
  (bind _returnvalue (UserInterface|CreateWidget "/Game/UI/TestLevel/StartMessage.StartMessage_C"))
  (UserInterface|Viewport|AddtoViewport _returnvalue 0))

(event Custom|AddKillToScore
  (bind _playerkd (Variables|Default|GetPlayerKD))
  ;[1 1 1] Add kill
  (Utilities|Struct|SetmembersinPlayerKD _playerkd (+ (.Kills (Utilities|Struct|BreakPlayerKD _playerkd)) 1)))

(event Custom|UpdateServer
  (params (CharacterInfo :type Player%20KD%20Structure) (StatusChanged? :type Boolean))
  ;[1 1 1] On server update player info
  (Variables|Default|SetPlayerKD CharacterInfo)
  (Default|SwapCharacter (.AsTest%20GM (Utilities|Casting|CastToTestGM (Game|GetGameMode))) self 0 StatusChanged?))

(event Custom|RemovePlayerList
  ;[1 1 1] Show / Hide player K/D
  (Widget|RemovefromParent (stale Custom|AddPlayerListWidget _returnvalue)))

(fn ConstructionScript)

(fn GetCharacterClassbyID
  (CallFunction|FillPlayerClass (Utilities|Array|Get(acopy) (Variables|/Game/Blueprints/TestBP/TestGM.TestGM_C|GetCharactersInClass (.AsTest%20GM (Utilities|Casting|CastToTestGM (Game|GetGameMode)))) (Variables|Default|GetCharacterID))))